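; Level element that catches player characters in a trigger and puts them into a falling-to-respawn state.
; On overlap with PlayerDecttor, a BP_Character not already flagged drops its carried actor and gets FallingToRespawn set.
; It also loses horizontal velocity while keeping vertical speed, and its PaperZD locomotion state machine jumps to the falling animation.
; The respawn itself is not handled here.
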(event OnComponentBeginOverlap(PlayerDecttor)
  (params (OverlappedComponent :type Primitive%20Component%20Object%20Reference) (OtherActor :type Actor%20Object%20Reference) (OtherComp :type Primitive%20Component%20Object%20Reference) (OtherBodyIndex :type Integer) (bFromSweep :type Boolean) (SweepResult :type Hit%20Result%20Structure%20%28by%20ref%29))
  (bind _asbp_character (Utilities|Casting|CastToBP_Character OtherActor))
  (if (not (Variables|/Game/Blueprints/BP_Character.BP_Character_C|GetfallingToRespawn _asbp_character))
    (Default|DropActor _asbp_character)
    (Variables|/Game/Blueprints/BP_Character.BP_Character_C|SetfallingToRespawn _asbp_character true)
    (Variables|/Script/Engine.MovementComponent|SetVelocity (Variables|/Script/Engine.Character|GetCharacterMovement _asbp_character) (Math|Vector|MakeVector 0.0 0.0 (.z (Variables|/Script/Engine.MovementComponent|GetVelocity (Variables|/Script/Engine.Character|GetCharacterMovement _asbp_character)))))
    (Class|PaperZDAnimInstance|JumptoNode (Variables|/Script/PaperZD.PaperZDAnimationComponent|GetAnimInstance (Variables|/Game/Blueprints/BP_Character.BP_Character_C|GetPaperZDAnimation _asbp_character)) "Falling_Jump" "LocomotionStateMachine")))

(event EventBeginPlay)

(event Collision|EventActorBeginOverlap
  (params (OtherActor :type Actor%20Object%20Reference)))

(event EventTick
  (params (DeltaSeconds :type Float%20%28single-precision%29)))

(fn ConstructionScript)