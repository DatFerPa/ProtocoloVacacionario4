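; Level element boot that kicks pickable actors entering its detection volume along the forward vector of its Direction component.
; An overlap triggers a kick timeline that swings the boot and fires an event applying the kick through BPI_IPickable, with a data-table sound.
; A cooldown timeline follows, then the boot becomes ready and repeats if pickable actors not currently being held still overlap.
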(event OnComponentBeginOverlap(DetectionCollision)
  (params (OverlappedComponent :type Primitive%20Component%20Object%20Reference) (OtherActor :type Actor%20Object%20Reference) (OtherComp :type Primitive%20Component%20Object%20Reference) (OtherBodyIndex :type Integer) (bFromSweep :type Boolean) (SweepResult :type Hit%20Result%20Structure%20%28by%20ref%29))
  (bind _detectioncollision (Variables|Default|GetDetectionCollision))
  (if (Variables|Default|GetisKickReady)
    (Variables|Default|SetisKickReady false)
    (|PerformingKick :!label _label
      (:Finished
        (Variables|Default|SetisKickReady true)
        (bind (_outactors _returnvalue) (Collision|ComponentOverlapActors _detectioncollision (Transformation|GetWorldTransform _detectioncollision) (Utilities|Array|MakeArray "ObjectTypeQuery4" "ObjectTypeQuery3") 0))
        (if _returnvalue
          (bind _array_element (Utilities|Array|ForEachLoopwithBreak _outactors)
            (:LoopBody
              (if (Utilities|DoesObjectImplementInterface _array_element "/Game/Blueprints/BPI_IPickable.BPI_IPickable_C")
                (bind _isactorkickeable (CallFunction|IsActorKickeable _array_element))
                (if _isactorkickeable
                  (goto _label))))))))))

(event EventBeginPlay)

(fn ConstructionScript)

(fn IsActorKickeable
  (params (actorToBeKicked :type Actor%20Object%20Reference))
  (if (Utilities|DoesObjectImplementInterface actorToBeKicked "/Game/Blueprints/BPI_IPickable.BPI_IPickable_C")
    (bind _isbeingpicked (Class|BPIIPickable|GetIsBeingPicked(Message) actorToBeKicked))
    (if _isbeingpicked
      (return false)
      (else
        (return true)))))

(fn KickEntitiesOverlaped
  (bind _detectioncollision (Variables|Default|GetDetectionCollision))
  (bind _outactors (Collision|ComponentOverlapActors _detectioncollision (Transformation|GetWorldTransform _detectioncollision) (Utilities|Array|MakeArray "ObjectTypeQuery4" "ObjectTypeQuery3") 0))
  (Utilities|FlowControl|Sequence
    (:then_0
      (bind _returnvalue (Utilities|GetDataTableRow "/Game/Audio/DT_Sound.DT_Sound" "KickBootKick")
        (:then
          (Audio|PlaySound2D (Utilities|Struct|BreakS_AudioRow _returnvalue) 1.0 1.0 0.0 0 0))))
    (:then_1
      (for _array_element _outactors
        (if (Utilities|DoesObjectImplementInterface _array_element "/Game/Blueprints/BPI_IPickable.BPI_IPickable_C")
          (Class|BPIIPickable|BeingKicked(Message) _array_element (Math|Vector|GetForwardVector (Variables|Default|GetDirection))))))))