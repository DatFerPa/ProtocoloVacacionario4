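; BP_Camera is a shared orthographic camera that keeps the characters in CharactersInGame framed by moving and zooming.
; Every Tick, GetNewPosition finds the XY bounding box of their capsules and snaps the actor to its center, keeping its Z.
; The farthest character's 2D distance from that center, clamped and normalized, linearly maps OrthoWidth between minimum and maximum, with no smoothing over time.
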(event EventBeginPlay)

(event Collision|EventActorBeginOverlap
  (params (OtherActor :type Actor%20Object%20Reference)))

(event EventTick
  (params (DeltaSeconds :type Float%20%28single-precision%29))
  (CallFunction|GetNewPosition))

(fn ConstructionScript)

(fn GetNewPosition
  (Variables|Default|SetCurrentMaxDistanceBetweenCameraAndFurderPlayer 0.0)
  (for (_array_element _array_index) (Variables|Default|GetCharactersInGame)
    (if (== _array_index 0)
      (Variables|Default|SetMinXPoint (.x (Transformation|GetWorldLocation (Variables|/Script/Engine.Character|GetCapsuleComponent _array_element))))
      (Variables|Default|SetMaxXPoint (.x (Transformation|GetWorldLocation (Variables|/Script/Engine.Character|GetCapsuleComponent _array_element))))
      (Variables|Default|SetMinYPoint (.y (Transformation|GetWorldLocation (Variables|/Script/Engine.Character|GetCapsuleComponent _array_element))))
      (Variables|Default|SetMaxYPoint (.y (Transformation|GetWorldLocation (Variables|/Script/Engine.Character|GetCapsuleComponent _array_element))))
      (else
        (if (<= (Variables|Default|GetMinXPoint) (.x (Transformation|GetWorldLocation (Variables|/Script/Engine.Character|GetCapsuleComponent _array_element))))
          _
          (else
            (Variables|Default|SetMinXPoint (.x (Transformation|GetWorldLocation (Variables|/Script/Engine.Character|GetCapsuleComponent _array_element))))))
        (if (>= (Variables|Default|GetMaxXPoint) (.x (Transformation|GetWorldLocation (Variables|/Script/Engine.Character|GetCapsuleComponent _array_element))))
          _
          (else
            (Variables|Default|SetMaxXPoint (.x (Transformation|GetWorldLocation (Variables|/Script/Engine.Character|GetCapsuleComponent _array_element))))))
        (if (<= (Variables|Default|GetMinYPoint) (.y (Transformation|GetWorldLocation (Variables|/Script/Engine.Character|GetCapsuleComponent _array_element))))
          _
          (else
            (Variables|Default|SetMinYPoint (.y (Transformation|GetWorldLocation (Variables|/Script/Engine.Character|GetCapsuleComponent _array_element))))))
        (if (not (>= (Variables|Default|GetMaxYPoint) (.y (Transformation|GetWorldLocation (Variables|/Script/Engine.Character|GetCapsuleComponent _array_element)))))
          (Variables|Default|SetMaxYPoint (.y (Transformation|GetWorldLocation (Variables|/Script/Engine.Character|GetCapsuleComponent _array_element))))))))
  (Variables|Default|SetPositionToCenter (Math|Vector|MakeVector (/ (+ (Variables|Default|GetMaxXPoint) (Variables|Default|GetMinXPoint)) 2.0) (/ (+ (Variables|Default|GetMinYPoint) (Variables|Default|GetMaxYPoint)) 2.0) 0.0))
  (for _array_element_2 (Variables|Default|GetCharactersInGame)
    (if (> (Math|Vector|Distance2D(Vector) (Variables|Default|GetPositionToCenter) (Transformation|GetWorldLocation (Variables|/Script/Engine.Character|GetCapsuleComponent _array_element_2))) (Variables|Default|GetCurrentMaxDistanceBetweenCameraAndFurderPlayer))
      (Variables|Default|SetCurrentMaxDistanceBetweenCameraAndFurderPlayer (Math|Vector|Distance2D(Vector) (Variables|Default|GetPositionToCenter) (Transformation|GetWorldLocation (Variables|/Script/Engine.Character|GetCapsuleComponent _array_element_2))))))
  (Transformation|SetActorLocation (Math|Vector|MakeVector (.x (Variables|Default|GetPositionToCenter)) (.y (Variables|Default|GetPositionToCenter)) (.z (Transformation|GetActorLocation))) false false)
  (Class|CameraComponent|SetOrthoWidth (Variables|CameraActor|GetCameraComponent) (Math|Float|Lerp (Variables|Default|GetMinOrthoWidth) (Variables|Default|GetMaxOrthoWidth) (Math|Float|NormalizetoRange (Math|Float|Clamp(Float) (Variables|Default|GetCurrentMaxDistanceBetweenCameraAndFurderPlayer) (Variables|Default|GetMinDistanceFromFurtherPlayer) (Variables|Default|GetMaxDistanceFromFurtherPlayer)) (Variables|Default|GetMinDistanceFromFurtherPlayer) (Variables|Default|GetMaxDistanceFromFurtherPlayer)))))