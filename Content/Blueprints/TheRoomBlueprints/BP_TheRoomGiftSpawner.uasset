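; Spawner actor for The Room that drops the gifts collected during the session into a box volume, one by one.
; On BeginPlay it caches the gift-information GameInstance and starts a short looping timer to pace spawning.
; SpawnGift creates each linked gift class and variation at half scale, with random position in SpawnBox and random rotation.
; The timer clears once every collected gift has spawned.
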(event EventBeginPlay
  (bind _asgi_gift_information (Utilities|Casting|CastToGI_GiftInformation (Game|GetGameInstance)))
  (Variables|Default|SetGiftInformation _asgi_gift_information)
  (bind _returnvalue (Utilities|Time|SetTimerbyEvent (EventDispatchers|CreateEvent :!event SpawnGift) 0.2 true))
  (Variables|Default|SetTimerToSpawn _returnvalue))

(fn ConstructionScript)

(fn SpawnGift
  (bind _returnvalue (Math|Random|RandomFloatinRange 0.0 3.6e+02))
  (bind _spawnbox (Variables|Default|GetSpawnBox))
  (bind _giftinformation (Variables|Default|GetGiftInformation))
  (bind _gifttospawn (Variables|Default|GetGiftToSpawn))
  (bind (_origin _boxextent) (Collision|GetComponentBounds _spawnbox))
  (bind _collectedgiftsduringsession (Variables|/Game/GameConfiguration/GI_GiftInformation.GI_GiftInformation_C|GetCollectedGiftsDuringSession _giftinformation))
  (bind _output (Utilities|Array|Get(acopy) _collectedgiftsduringsession _gifttospawn))
  (if (> (Utilities|Array|Length _collectedgiftsduringsession) (Variables|Default|GetGiftToSpawn))
    (Game|SpawnActorfromClass (.linkedgift _output) (Math|Transform|MakeTransform (Math|Random|RandomPointinBoundingBox _origin _boxextent) (Math|Rotator|MakeRotator _returnvalue _returnvalue _returnvalue) "0.500000,0.500000,0.500000") "Undefined" "OverrideRootScale" 0 (.giftvariation _output) 0)
    (Math|Integer|IncrementInt (Variables|Default|GetGiftToSpawn))
    (else
      (Utilities|Time|ClearandInvalidateTimerbyHandle (Variables|Default|GetTimerToSpawn)))))