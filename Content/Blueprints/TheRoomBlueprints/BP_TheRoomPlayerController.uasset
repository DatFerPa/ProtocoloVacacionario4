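; Player controller for TheRoom, viewing through a level camera while the player steers an on-screen crosshair and shoots physics impulses.
; Cursor input moves a stored viewport position and the crosshair widget, which CreateWidgetCrosshair builds and returns.
; Shooting deprojects that offset position, traces from the camera with debug drawing, then teleports a radial force to the impact and fires it.
; A back-to-menu input opens 01_TestingMap.
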(event Input|EnhancedActionEvents|EnhancedInputActionIA_BackToMainMenu
  (params (ActionValue :type Boolean) (ElapsedSeconds :type Float%20%28double-precision%29) (TriggeredSeconds :type Float%20%28double-precision%29) (InputAction :type Input%20Action%20Object%20Reference :default "/Game/GameConfiguration/Inputs/TheRoomInputs/Actions/IA_BackToMainMenu.IA_BackToMainMenu"))
  (Game|OpenLevel(byObjectReference) "/Game/Maps/01_TestingMap.01_TestingMap"))

(event Input|EnhancedActionEvents|EnhancedInputActionIA_MoveCursor
  (params (ActionValue :type Vector%202D%20Structure) (ElapsedSeconds :type Float%20%28double-precision%29) (TriggeredSeconds :type Float%20%28double-precision%29) (InputAction :type Input%20Action%20Object%20Reference :default "/Game/GameConfiguration/Inputs/TheRoomInputs/Actions/IA_MoveCursor.IA_MoveCursor"))
  (bind _output_get (Variables|Default|SetviewPortPosition (+ (Variables|Default|GetviewPortPosition) (* ActionValue (Variables|Default|GetMovementFactor)))))
  (Default|MovetoNewPosition (Variables|Default|GetLinkedCrosshair) _output_get))

(event Input|EnhancedActionEvents|EnhancedInputActionIA_Shoot
  (params (ActionValue :type Boolean) (ElapsedSeconds :type Float%20%28double-precision%29) (TriggeredSeconds :type Float%20%28double-precision%29) (InputAction :type Input%20Action%20Object%20Reference :default "/Game/GameConfiguration/Inputs/TheRoomInputs/Actions/IA_Shoot.IA_Shoot"))
  (bind _returnvalue (Game|GetPlayerController 0))
  (bind _viewportposition (Variables|Default|GetviewPortPosition))
  (bind _radialforce (Variables|Default|GetRadialForce))
  (bind _returnvalue_2 (+ (.y _viewportposition) 5e+01))
  (bind _returnvalue_3 (+ (.x _viewportposition) 5e+01))
  (bind (_worldlocation _worlddirection) (Class|PlayerController|DeprojectScreenPositiontoWorld _returnvalue _returnvalue_3 _returnvalue_2))
  (:Triggered
    (bind _outhit (Collision|LineTraceByChannel (Transformation|GetWorldLocation (Variables|/Script/Engine.Actor|GetRootComponent (Variables|Default|GetReferencedCamera))) (+ _worldlocation (* _worlddirection 1e+03)) "TraceTypeQuery1" false 0 "ForDuration"))
    (Rendering|Debug|DrawDebugSphere (.location _outhit) 1e+02 12 "(R=1.000000,G=0.000000,B=0.720168,A=1.000000)" 2.0 2.0)
    (Transformation|SetWorldLocation _radialforce (.impactpoint _outhit) false true)
    (Class|RadialForceComponent|FireImpulse _radialforce)))

(event EventBeginPlay
  (bind _self self)
  (bind _returnvalue (PlayerController|LocalPlayerSubsystems|GetEnhancedInputLocalPlayerSubsystem _self))
  (Utilities|FlowControl|Sequence
    (:then_0
      ;[0.2549 0.2549 0.2549] Adding Input Mapping
      (Utilities|FlowControl|Delay 0.2)
      (Utilities|IsValid _returnvalue
        (:Is%20Valid
          (Input|AddMappingContext _returnvalue "/Game/GameConfiguration/Inputs/TheRoomInputs/IMC_TheRoom.IMC_TheRoom" 0 "(bIgnoreAllPressedKeysUntilRelease=True,bForceImmediately=False,bNotifyUserSettings=False)"))))
    (:then_1
      (bind _returnvalue_2 (Actor|GetActorOfClass "/Script/Engine.CameraActor"))
      (bind _output_get (Variables|Default|SetReferencedCamera _returnvalue_2))
      (Game|Player|SetViewTargetwithBlend _output_get 0.0 "VTBlend_Linear" 0.0 false))))

(fn ConstructionScript)

(fn CreateWidgetCrosshair
  (bind _returnvalue (UserInterface|CreateWidget "/Game/UI/UI_TheRoom/WBP_Crosshair.WBP_Crosshair_C" 0 self))
  (bind _output_get (Variables|Default|SetLinkedCrosshair _returnvalue))
  (UserInterface|Viewport|AddtoViewport _returnvalue 0)
  (Class|UserWidget|SetPositioninViewport :self _returnvalue)
  (return _output_get))