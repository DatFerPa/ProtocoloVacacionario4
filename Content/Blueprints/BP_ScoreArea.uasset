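; BP_ScoreArea is a trigger box that scores gifts dropped into it in the Holiday Protocol game mode.
; On BeginPlay it caches a reference to GM_HolidayProtocolGameMode.
; When a BP_Gift overlaps the box, it calls CashGift on the game mode unless that gift is already in AlreadyCashedGifts, preventing double scoring.
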(event OnComponentBeginOverlap(Box)
  (params (OverlappedComponent :type Primitive%20Component%20Object%20Reference) (OtherActor :type Actor%20Object%20Reference) (OtherComp :type Primitive%20Component%20Object%20Reference) (OtherBodyIndex :type Integer) (bFromSweep :type Boolean) (SweepResult :type Hit%20Result%20Structure%20%28by%20ref%29))
  (bind _asbp_gift (Utilities|Casting|CastToBP_Gift OtherActor))
  (if (not (Utilities|Array|ContainsItem (Variables|/Game/GameConfiguration/GM_HolidayProtocolGameMode.GM_HolidayProtocolGameMode_C|GetAlreadyCashedGifts (Variables|Default|GetGameMode)) _asbp_gift))
    (Default|CashGift (Variables|Default|GetGameMode) _asbp_gift)))

(event EventBeginPlay
  (bind _asgm_holiday_protocol_game_mode (Utilities|Casting|CastToGM_HolidayProtocolGameMode (Game|GetGameMode)))
  (Variables|Default|SetGameMode _asgm_holiday_protocol_game_mode))

(fn ConstructionScript)