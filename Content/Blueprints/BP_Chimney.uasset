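; BP_Chimney is a chimney actor that periodically spits out gifts.
; Its construction script fills the gift list from data table rows, which is shuffled at BeginPlay and whenever exhausted.
; A looping timer, with its interval randomized once, spawns each gift inside SpawnBox and kicks it away from CenterPoint through BPI_IPickable.
; A random starting count varies how many spawn before the timer stops, unless infinite spawning is enabled.
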(event Custom|SpawnPresents
  (bind _returnvalue (Math|Random|RandomFloatinRange 0.0 3.6e+02))
  (bind _giftstospawn (Variables|Default|GetGiftsToSpawn))
  (bind _spawnbox (Variables|Default|GetSpawnBox))
  (bind _currentpresent (Variables|Default|GetCurrentPresent))
  (bind (_origin _boxextent) (Collision|GetComponentBounds _spawnbox))
  (bind _output (Utilities|Array|Get(acopy) _giftstospawn _currentpresent))
  (CallFunction|ReShuffleLogic)
  (bind _returnvalue_2 (Game|SpawnActorfromClass (.linkedgift _output) (Math|Transform|MakeTransform (Math|Random|RandomPointinBoundingBox _origin _boxextent) (Math|Rotator|MakeRotator _returnvalue _returnvalue _returnvalue) (Variables|Default|GetGiftScale)) "Undefined" "OverrideRootScale" 0 (.giftvariation _output) 0))
  (CallFunction|LaunchGift _returnvalue_2)
  (Math|Integer|IncrementInt (Variables|Default|GetCurrentPresent)
    (:%20%20
      (Math|Integer|IncrementInt (Variables|Default|GetAccumulatedSpawnedPresents)
        (:%20%20
          (if (and (>= (Variables|Default|GetAccumulatedSpawnedPresents) (Variables|Default|GetMaxPresentsToSpawn)) (not (Variables|Default|GetisInifniteSpawn)))
            (Utilities|Time|ClearandInvalidateTimerbyHandle (stale EventBeginPlay _returnvalue))))))))

(event EventBeginPlay
  (Utilities|Array|Shuffle (Variables|Default|GetGiftsToSpawn))
  (Variables|Default|SetAccumulatedSpawnedPresents (Math|Random|RandomInteger (Variables|Default|GetMaxPresentsToSpawn)))
  (bind _returnvalue (Utilities|Time|SetTimerbyEvent (delegate Custom|SpawnPresents) (Math|Random|RandomFloatinRange (Variables|Default|GetMinDelayBetweenPresent) (Variables|Default|GetMaxDelayBetweenPresent)) true)))

(fn ConstructionScript
  (for _array_element (Variables|Default|GetGiftsToSpawn_DT)
    (bind _returnvalue (Utilities|GetDataTableRow (.datatable _array_element) (.rowname _array_element))
      (:then
        (Utilities|Array|Add (Variables|Default|GetGiftsToSpawn) _returnvalue)))))

(fn ReShuffleLogic
  (if (>= (Variables|Default|GetCurrentPresent) (Utilities|Array|Length (Variables|Default|GetGiftsToSpawn)))
    (Utilities|Array|Shuffle (Variables|Default|GetGiftsToSpawn))
    (Variables|Default|SetCurrentPresent 0)))

(fn LaunchGift
  (params (GiftToLaunch :type BP%20Gift%20Object%20Reference))
  (if (Utilities|DoesObjectImplementInterface GiftToLaunch "/Game/Blueprints/BPI_IPickable.BPI_IPickable_C")
    (Default|BeingKicked GiftToLaunch (* (Math|Vector|Normalize (- (Transformation|GetWorldLocation (Variables|/Game/Blueprints/BP_Gift.BP_Gift_C|GetGiftMesh GiftToLaunch)) (Transformation|GetWorldLocation (Variables|Default|Getcenter%20Point)))) (Variables|Default|GetPushWhenSpawningFactor)))))