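; BP_Gift is a gift actor that can be picked up, dropped and kicked.
; Its construction script sets the mesh material from an array by variation index.
; Pick, drop and kick events call TogglePhysics to switch simulation and collision together, with kicks adding a scaled velocity-change impulse.
; A separate getter and setter expose the IsPicked flag, which these events leave untouched.
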(event EventBeginPlay)

(event Collision|EventActorBeginOverlap
  (params (OtherActor :type Actor%20Object%20Reference)))

(event EventBeingDropped
  (CallFunction|TogglePhysics true))

(event EventBeingKicked
  (params (ForceVector :type Vector :default "0, 0, 0"))
  (CallFunction|TogglePhysics true)
  (Physics|AddImpulse (Variables|Default|GetGiftMesh) (* ForceVector (Variables|Default|GetKickForce)) "None" true))

(event EventBeingPicked
  (CallFunction|TogglePhysics false))

(fn ConstructionScript
  (Rendering|Material|SetMaterial (Variables|Default|GetGiftMesh) 0 (Utilities|Array|Get(acopy) (Variables|Default|GetMaterials) (Variables|Default|GetGiftVariationToUse))))

(fn TogglePhysics
  (params (isSimulatingPhysics :type Boolean))
  (bind _giftmesh (Variables|Default|GetGiftMesh))
  (if isSimulatingPhysics
    (Physics|SetSimulatePhysics _giftmesh true)
    (Collision|SetCollisionEnabled _giftmesh "QueryAndPhysics")
    (else
      (Physics|SetSimulatePhysics _giftmesh false)
      (Collision|SetCollisionEnabled _giftmesh "NoCollision"))))

(fn GetIsBeingPicked
  (return (Variables|Default|GetisPicked)))

(fn SetIsBeingPicked
  (params (inputIsBeingPicked :type Boolean))
  (bind _output_get (Variables|Default|SetisPicked inputIsBeingPicked))
  (return _output_get))