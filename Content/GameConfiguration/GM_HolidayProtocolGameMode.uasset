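; Game mode for a local multiplayer gift-delivery level, handling player creation, shared camera, score, countdown, respawn points and level end.
; BP_LevelManager supplies level time and a shuffled gift list that randomly refills a capped request queue.
; CashGift matches gift class and variation against that queue to award points.
; Near zero, the countdown switches to slower ticks, then EndLevel shows results and saves cashed gifts to the game instance.
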(event EventBeginPlay
  (Utilities|FlowControl|Sequence
    (:then_0
      ;[0.2549 0.2549 0.2549] Creation and configuration of the local Players
      (bind (_outusers _returnvalue) (Class|InputDeviceLibrary|GetAllActiveUsers))
      (Development|PrintString (Utilities|String|Append "Amount of Detected Players: " (Utilities|String|ToString(Integer) _returnvalue)))
      (for (_array_element _array_index) _outusers
        (if (Utilities|IsValid (Class|GameplayStatics|GetPlayerControllerfromPlatformUser _array_element))
          (bind _asbp_character (Utilities|Casting|CastToBP_Character (Pawn|GetControlledPawn (Class|GameplayStatics|GetPlayerControllerfromPlatformUser _array_element))))
          (Variables|/Game/Blueprints/BP_Character.BP_Character_C|SetPlayerIndex _asbp_character _array_index)
          (else
            (bind _returnvalue_2 (Class|GameplayStatics|CreatePlayerfromPlatformUser _array_element))
            (bind _asbp_character_2 (Utilities|Casting|CastToBP_Character (Pawn|GetControlledPawn _returnvalue_2)))
            (Variables|/Game/Blueprints/BP_Character.BP_Character_C|SetPlayerIndex _asbp_character_2 _array_index)))))
    (:then_1
      ;[0.2549 0.2549 0.2549] Add the created Players to the camera in order to allow it to follow the Players
      (bind _returnvalue_3 (Actor|GetActorOfClass "/Game/Blueprints/BP_Camera.BP_Camera_C"))
      (bind _outactors (Actor|GetAllActorsOfClass "/Game/Blueprints/BP_Character.BP_Character_C"))
      (bind _output_get (Variables|/Game/Blueprints/BP_Camera.BP_Camera_C|SetCharactersInGame _returnvalue_3 _outactors))
      (for _array_element_2 _output_get
        (bind _asplayer_controller (Utilities|Casting|CastToPlayerController (Pawn|GetController _array_element_2)))
        (Game|Player|SetViewTargetwithBlend _asplayer_controller _returnvalue_3 0.0 "VTBlend_Linear" 0.0 false)
        (EventDispatchers|BindEventtoAnyKeytoEndLevel _array_element_2 (EventDispatchers|CreateEvent :!event ChangetoMainMenu))))
    (:then_2
      (bind _returnvalue_4 (UserInterface|CreateWidget "/Game/UI/HUD.HUD_C" 0 0))
      (Variables|/Game/UI/HUD.HUD_C|SetGameMode _returnvalue_4 self)
      (UserInterface|Viewport|AddtoViewport _returnvalue_4 0)
      (Default|CallOnScoreChanged))
    (:then_3
      ;[0.2549 0.2549 0.2549] Capturing the Information of the Level
      (bind _returnvalue_5 (Actor|GetActorOfClass "/Game/GameConfiguration/BP_LevelManager.BP_LevelManager_C"))
      (bind _gitstoask (Default|GetGiftstoAsk _returnvalue_5))
      (bind _output_get_2 (Variables|Default|SetGiftsToASk _gitstoask))
      (Utilities|Array|Shuffle _output_get_2)
      (bind _leveltime (Class|BPIHolidayProtocolLevelInformation|GetLevelTime(Message) _returnvalue_5))
      (Variables|Default|SetLevelTime _leveltime)
      (Default|CallOnTimeChange)
      (Variables|Default|SetMaxAmountOfQueueGifts (Variables|/Game/GameConfiguration/BP_LevelManager.BP_LevelManager_C|GetmaxAmountOfAskedGifts _returnvalue_5)))
    (:then_4
      (bind _returnvalue_6 (Utilities|Time|SetTimerbyEvent (EventDispatchers|CreateEvent :!event TimerLogic) 1.0 true))
      (Variables|Default|SetNormalTimer _returnvalue_6))
    (:then_5
      ;[0.2549 0.2549 0.2549] Seeting the Player Starts when respawning
      (bind _outactors_2 (Actor|GetAllActorsOfClass "/Script/Engine.PlayerStart"))
      (bind _output_get_3 (Variables|Default|SetPlayerStarts _outactors_2))
      (Utilities|Array|Shuffle _output_get_3))))

(fn ConstructionScript)

(fn ChangeScore
  (params (ChangeInScore :type Integer))
  (Variables|Default|SetScore (Math|Integer|Clamp(Integer) (+ ChangeInScore (Variables|Default|GetScore)) 0 2147483647))
  (Default|CallOnScoreChanged))

(fn CashGift
  (params (Gift :type BP%20Gift%20Object%20Reference))
  (bind _askedgifts (Variables|Default|GetAskedGifts))
  (bind (_array_element _array_index) (Utilities|Array|ForEachLoopwithBreak (Variables|Default|GetAskedGifts) :!label _label)
    (:LoopBody
      (if (and (== (.linkedgift _array_element) (Utilities|GetClass Gift)) (== (.giftvariation _array_element) (Variables|/Game/Blueprints/BP_Gift.BP_Gift_C|GetGiftVariationToUse Gift)))
        (LocalVariables|SetIndexToRemove _array_index)
        (goto _label Break)))
    (:Completed
      (if (!= (LocalVariables|GetIndexToRemove) -1)
        (bind _returnvalue (Utilities|GetDataTableRow "/Game/Audio/DT_Sound.DT_Sound" "RightGift")
          (:then
            (Audio|PlaySound2D (Utilities|Struct|BreakS_AudioRow _returnvalue) 1.0 1.0 0.0 0 0)
            (Utilities|Array|RemoveIndex _askedgifts (LocalVariables|GetIndexToRemove))
            (Default|CallUpdateGiftQueue _askedgifts)
            (Utilities|Array|Add (Variables|Default|GetAlreadyCashedGifts) (Utilities|Struct|MakeSTR_GiftInformationDataStructure (Utilities|GetClass Gift) (Variables|/Game/Blueprints/BP_Gift.BP_Gift_C|GetGiftVariationToUse Gift) 0 0))
            (CallFunction|ChangeScore (Variables|/Game/Blueprints/BP_Gift.BP_Gift_C|GetScorePoints Gift))))
        (else
          (bind _returnvalue_2 (Utilities|GetDataTableRow "/Game/Audio/DT_Sound.DT_Sound" "WrongGift")
            (:then
              (Audio|PlaySound2D (Utilities|Struct|BreakS_AudioRow _returnvalue_2) 1.0 1.0 0.0 0 0))))))))

(fn AddNewGift
  (bind _askedgifts (Variables|Default|GetAskedGifts))
  (if (< (Utilities|Array|Length (Variables|Default|GetAskedGifts)) (Variables|Default|GetMaxAmountOfQueueGifts))
    (bind _returnvalue (Utilities|GetDataTableRow "/Game/Audio/DT_Sound.DT_Sound" "NewGiftRequest")
      (:then
        (Audio|PlaySound2D (Utilities|Struct|BreakS_AudioRow _returnvalue) 1.0 1.0 0.0 0 0))
      (:RowNotFound
        _))
    (if (>= (Variables|Default|GetCurrentAskedGift) (Utilities|Array|Length (Variables|Default|GetGiftsToASk)))
      (Variables|Default|SetCurrentAskedGift 0)
      (Utilities|Array|Shuffle (Variables|Default|GetGiftsToASk)))
    (Utilities|Array|Add _askedgifts (Utilities|Array|Get(acopy) (Variables|Default|GetGiftsToASk) (Variables|Default|GetCurrentAskedGift)))
    (Default|CallUpdateGiftQueue _askedgifts)
    (Math|Integer|IncrementInt (Variables|Default|GetCurrentAskedGift))))

(fn EndLevel
  (Utilities|Array|Clear (Variables|Default|GetAskedGifts))
  (Viewport|RemoveAllWidgets)
  (bind _asgi_gift_information (Utilities|Casting|CastToGI_GiftInformation (Game|GetGameInstance))
    (:then
      (Default|StopGameplayBackgroundMusic _asgi_gift_information))
    (:CastFailed
      _))
  (bind _returnvalue (Actor|GetActorOfClass "/Game/GameConfiguration/BP_LevelManager.BP_LevelManager_C"))
  (bind _returnvalue_2 (UserInterface|CreateWidget "/Game/UI/WBP_LevelEnd.WBP_LevelEnd_C"))
  (Variables|/Game/UI/WBP_LevelEnd.WBP_LevelEnd_C|SetGameMode _returnvalue_2 self)
  (Variables|/Game/UI/WBP_LevelEnd.WBP_LevelEnd_C|SetNormalScoreAmount _returnvalue_2 (Variables|/Game/GameConfiguration/BP_LevelManager.BP_LevelManager_C|GetNormalScoreThreshold _returnvalue))
  (Variables|/Game/UI/WBP_LevelEnd.WBP_LevelEnd_C|SetGoodScoreAmount _returnvalue_2 (Variables|/Game/GameConfiguration/BP_LevelManager.BP_LevelManager_C|GetGoodScoreThreshold _returnvalue))
  (UserInterface|Viewport|AddtoViewport _returnvalue_2 0)
  (bind _outactors (Actor|GetAllActorsOfClass "/Game/Blueprints/BP_Character.BP_Character_C"))
  (for _array_element _outactors
    (bind _asplayer_controller (Utilities|Casting|CastToPlayerController (Pawn|GetController _array_element)))
    (Class|EnhancedInputSubsystemInterface|ClearAllMappings(Message) (PlayerController|LocalPlayerSubsystems|GetEnhancedInputLocalPlayerSubsystem _asplayer_controller))
    (Input|AddMappingContext (PlayerController|LocalPlayerSubsystems|GetEnhancedInputLocalPlayerSubsystem _asplayer_controller) "/Game/GameConfiguration/Inputs/MenusInputs/IMC_Menus.IMC_Menus" 0 "(bIgnoreAllPressedKeysUntilRelease=True,bForceImmediately=False,bNotifyUserSettings=False)"))
  (Variables|Default|SetisLevelEnded true)
  (CallFunction|CollectCashedGifts)
  (Default|CallEndLevelDispatcher))

(fn TimerLogic
  (bind _leveltime (Variables|Default|GetLevelTime))
  (Math|Integer|DecrementInt _leveltime
    (:%20%20
      (if (>= (Variables|Default|GetFromTimeToSlow) _leveltime)
        (Default|CallOnSlowmoTimeChange)
        (Utilities|Time|ClearandInvalidateTimerbyHandle (Variables|Default|GetNormalTimer))
        (bind _returnvalue (Utilities|Time|SetTimerbyEvent (EventDispatchers|CreateEvent :!event SlowmoTimerLogic) 1.5 true))
        (Variables|Default|SetSlowmoTimer _returnvalue)
        (else
          (Default|CallOnTimeChange)
          (CallFunction|LogicAmountOfGiftstoAsk))))))

(fn SlowmoTimerLogic
  (bind _leveltime (Variables|Default|GetLevelTime))
  (Math|Integer|DecrementInt _leveltime
    (:%20%20
      (Default|CallOnSlowmoTimeChange)
      (if (<= _leveltime 0)
        (Development|PrintString "Game Ends")
        (Utilities|Time|ClearandInvalidateTimerbyHandle (Variables|Default|GetSlowmoTimer))
        (CallFunction|EndLevel)
        (else
          (bind _returnvalue (Utilities|GetDataTableRow "/Game/Audio/DT_Sound.DT_Sound" "CountdownTickSound")
            (:then
              (Audio|PlaySound2D (Utilities|Struct|BreakS_AudioRow _returnvalue) 1.0 1.0 0.0 0 0))
            (:RowNotFound
              _))
          (CallFunction|LogicAmountOfGiftstoAsk))))))

(fn LogicAmountOfGiftstoAsk
  (if (<= (Utilities|Array|Length (Variables|Default|GetAskedGifts)) 0)
    (for _index (range 0 (Math|Random|RandomIntegerinRange 1 (Variables|Default|GetMaxAmountOfQueueGifts)))
      (CallFunction|AddNewGift))
    (elif (Math|Random|RandomBoolwithWeight 0.2)
      (CallFunction|AddNewGift))))

(fn ChangetoMainMenu
  (Utilities|FlowControl|DoOnce false
    (:Completed
      (Game|OpenLevel(byObjectReference) "/Game/Maps/00_MainMenu.00_MainMenu"))))

(fn CollectCashedGifts
  (bind _asgi_gift_information (Utilities|Casting|CastToGI_GiftInformation (Game|GetGameInstance)))
  (for _array_element (Variables|Default|GetAlreadyCashedGifts)
    (Utilities|Array|Add (Variables|/Game/GameConfiguration/GI_GiftInformation.GI_GiftInformation_C|GetCollectedGiftsDuringSession _asgi_gift_information) _array_element)))

(fn GetPlayerRespawn
  (bind _playerstarts (Variables|Default|GetPlayerStarts))
  (Math|Integer|IncrementInt (Variables|Default|GetCurrentPlayerStartRespawn)
    (:%20%20
      (if (>= (Variables|Default|GetCurrentPlayerStartRespawn) (Utilities|Array|Length (Variables|Default|GetPlayerStarts)))
        (Utilities|Array|Shuffle _playerstarts)
        (Variables|Default|SetCurrentPlayerStartRespawn 0))
      (return (Utilities|Array|Get(acopy) _playerstarts (Variables|Default|GetCurrentPlayerStartRespawn))))))