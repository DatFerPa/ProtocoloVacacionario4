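; GM_TheRoom is the game mode for TheRoom that sets up the HUD and local multiplayer players at BeginPlay.
; It creates the TheRoom HUD widget, stores it and adds it to the viewport.
; It then iterates all active platform users, reusing the existing controller for the first and spawning a local player for each additional one.
; Each resulting BP_TheRoomPlayerController creates its own crosshair widget.
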(event EventBeginPlay
  (Utilities|FlowControl|Sequence
    (:then_0
      (bind _returnvalue (UserInterface|CreateWidget "/Game/UI/UI_TheRoom/HUD_TheRoom.HUD_TheRoom_C"))
      (Variables|Default|SetTheRoomHUD _returnvalue)
      (UserInterface|Viewport|AddtoViewport _returnvalue 0))
    (:then_1
      ;[0.2549 0.2549 0.2549] Create local Players
      (bind (_outusers _returnvalue_2) (Class|InputDeviceLibrary|GetAllActiveUsers))
      (Development|PrintString (Utilities|String|Append "Amount of Detected Players: " (Utilities|String|ToString(Integer) _returnvalue_2)))
      (for (_array_element _array_index) _outusers
        (if (== _array_index 0)
          (bind _returnvalue_3 (Class|InputDeviceLibrary|GetPlayerControllerfromPlatformUser _array_element))
          (bind _asbp_the_room_player_controller (Utilities|Casting|CastToBP_TheRoomPlayerController _returnvalue_3))
          (Default|CreateWidgetCrosshair _asbp_the_room_player_controller)
          (else
            (bind _returnvalue_4 (Class|GameplayStatics|CreatePlayerfromPlatformUser _array_element))
            (bind _asbp_the_room_player_controller_2 (Utilities|Casting|CastToBP_TheRoomPlayerController _returnvalue_4))
            (Default|CreateWidgetCrosshair _asbp_the_room_player_controller_2)))))))

(fn ConstructionScript)