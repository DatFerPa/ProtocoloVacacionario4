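; BP_LevelManager holds per-level configuration for gift requests: the gifts to ask for, the level time and the maximum number of asked gifts.
; GetGiftsToAsk resolves the level's list of Data Table row references into gift rows, skips any not found, and returns the collected array.
; Simple getters expose the time and maximum, and the event graph has no active logic.
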(event EventBeginPlay)

(event Collision|EventActorBeginOverlap
  (params (OtherActor :type Actor%20Object%20Reference)))

(event EventTick
  (params (DeltaSeconds :type Float%20%28single-precision%29)))

(fn ConstructionScript)

(fn GetGiftstoAsk
  (for _array_element (Variables|Default|GetgiftsToAskAtTheLevel)
    (bind _returnvalue (Utilities|GetDataTableRow (.datatable _array_element) (.rowname _array_element))
      (:then
        (Utilities|Array|Add (LocalVariables|GetGiftsToSend) _returnvalue))))
  (return (LocalVariables|GetGiftsToSend)))

(fn GetLevelTime
  (return (Variables|Default|GetlevelTime)))

(fn GetMaxAmountOfAskedGifts
  (return (Variables|Default|GetmaxAmountOfAskedGifts)))